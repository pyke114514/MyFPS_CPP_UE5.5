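; FPS player controller that creates and drives the player's crosshair, player, feedback and match-state HUD widgets.
; Looping timers poll until the pawn is known before creating widgets, and until PlayerState and StateHUD exist to seed the scoreboard.
; Tick pushes match time and phase, and detects pawn changes to notify widgets of respawns.
; A GameState scoreboard event refreshes player stats and the cached scoreboard.
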(event Custom|Client_DrawHUD
  (bind _returnvalue (Utilities|Time|SetTimerbyEvent (delegate Custom|HandleClient_DrawHUD) 0.1 true))
  (Variables|Default|SetTimer1 _returnvalue))

(event Custom|HandleClient_DrawHUD
  (if (Utilities|IsValid (Variables|Default|GetCurrentPlayer))
    (Utilities|Time|ClearandInvalidateTimerbyHandle (Variables|Default|GetTimer1))
    (bind _returnvalue (UserInterface|CreateWidget "/Game/MyAssets/HUD/WBP_CrosshairHUD.WBP_CrosshairHUD_C"))
    (bind _output_get (Variables|Default|SetCrosshairHUD _returnvalue))
    (UserInterface|Viewport|AddtoViewport _output_get 0)
    (bind _returnvalue_2 (UserInterface|CreateWidget "/Game/MyAssets/HUD/WBP_PlayerHUD.WBP_PlayerHUD_C"))
    (bind _output_get_2 (Variables|Default|SetPlayerHUD _returnvalue_2))
    (UserInterface|Viewport|AddtoViewport _output_get_2 0)
    (bind _returnvalue_3 (UserInterface|CreateWidget "/Game/MyAssets/HUD/WBP_FeedbackHUD.WBP_FeedbackHUD_C"))
    (bind _output_get_3 (Variables|Default|SetFeedbackHUD _returnvalue_3))
    (UserInterface|Viewport|AddtoViewport _output_get_3 0)
    (Default|HUDAvalable (Variables|Default|GetCurrentPlayer))
    (bind _returnvalue_4 (UserInterface|CreateWidget "/Game/MyAssets/HUD/WBP_StateHUD.WBP_StateHUD_C"))
    (bind _output_get_4 (Variables|Default|SetStateHUD _returnvalue_4))
    (UserInterface|Viewport|AddtoViewport _output_get_4 0)))

(event Custom|OnScoreBoardUpdated_BP
  (bind _statehud (Variables|Default|GetStateHUD))
  (bind _myplayerstate (Variables|Default|GetMyPlayerState))
  (Utilities|IsValid _statehud
    (:Is%20Valid
      (Default|UpdatePlayerStats _statehud (Variables|/Script/Engine.PlayerState|GetScore _myplayerstate) (Class|MyFPSCPPPlayerState|GetKills _myplayerstate) (Class|MyFPSCPPPlayerState|GetDeaths _myplayerstate))
      (Default|UpdateScoreboard _statehud (Class|MyFPSCPPGameState|GetCachedScoreboard (Variables|Default|GetMyGameState))))))

(event Custom|TryGetPlayerState
  (bind _mygamestate (Variables|Default|GetMyGameState))
  (bind _statehud (Variables|Default|GetStateHUD))
  (bind _asmy_fps_cppplayer_state (Utilities|Casting|CastToMyFPS_CPPPlayerState (Variables|Default|GetPlayerState)))
  (Variables|Default|SetMyPlayerState _asmy_fps_cppplayer_state)
  (EventDispatchers|BindEventtoOnScoreboardUpdated _mygamestate (delegate Custom|OnScoreBoardUpdated_BP))
  (Utilities|IsValid _statehud
    (:Is%20Valid
      (Default|UpdateScoreboard _statehud (Class|MyFPSCPPGameState|GetCachedScoreboard _mygamestate))
      (Utilities|Time|ClearandInvalidateTimerbyHandle (Variables|Default|GetTimer2)))))

(event EventTick
  (params (DeltaSeconds :type Float%20%28single-precision%29))
  (bind _feedbackhud (Variables|Default|GetFeedbackHUD))
  (bind _mygamestate (Variables|Default|GetMyGameState))
  (bind _statehud (Variables|Default|GetStateHUD))
  (bind _playerhud (Variables|Default|GetPlayerHUD))
  (bind _crosshairhud (Variables|Default|GetCrosshairHUD))
  (Utilities|IsValid _statehud
    (:Is%20Valid
      (Default|UpdateMatchTime _statehud (Class|MyFPSCPPGameState|GetRemainingTime _mygamestate))
      (Default|UpdateMatchPhase _statehud (Class|MyFPSCPPGameState|GetMatchPhase _mygamestate)))
    (:Is%20Not%20Valid
      _))
  (bind _asbp_first_person_character (Utilities|Casting|CastToBP_FirstPersonCharacter (Pawn|GetControlledPawn)))
  (if (!= _asbp_first_person_character (Variables|Default|GetCurrentPlayer))
    (Variables|Default|SetCurrentPlayer _asbp_first_person_character)
    (if (Utilities|IsValid _playerhud)
      (Default|PlayerRespawned _playerhud (Variables|Default|GetCurrentPlayer))
      (if (Utilities|IsValid _crosshairhud)
        (Default|PlayerRespawned _crosshairhud (Variables|Default|GetCurrentPlayer))
        (if (Utilities|IsValid _feedbackhud)
          (Default|PlayerRespawned _feedbackhud (Variables|Default|GetCurrentPlayer)))))))

(event EventBeginPlay
  (bind _asmy_fps_cppgame_state (Utilities|Casting|CastToMyFPS_CPPGameState (Game|GetGameState)))
  (Variables|Default|SetMyGameState _asmy_fps_cppgame_state)
  (bind _asmy_fps_cppgame_instance (Utilities|Casting|CastToMyFPS_CPPGameInstance (Game|GetGameInstance)))
  (Variables|Default|SetMyGameInstance _asmy_fps_cppgame_instance)
  (bind _returnvalue (Utilities|Time|SetTimerbyEvent (delegate Custom|TryGetPlayerState) 0.1 true))
  (Variables|Default|SetTimer2 _returnvalue))

(fn ConstructionScript)