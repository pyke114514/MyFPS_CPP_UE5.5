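; AI-controlled FPS character that mirrors its player-detection state into the AI blackboard.
; A setup event caches the AI controller and blackboard, and binds score changes on its player state to clear detection and target.
; Perception updates and Tick share one path writing the detected flag and target actor to the blackboard.
; Tick also clears detection and stops firing when the target is invalid.
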(event OnPerceptionUpdated(PerceptionComponent)
  (params (UpdatedActors :type Array%20of%20Actor%20Object%20References))
  (bind _blackboard (Variables|Default|GetBlackBoard))
  (Utilities|IsValid _blackboard
    (:Is%20Valid
      (AI|Components|Blackboard|SetValueasBool _blackboard (Utilities|Name|MakeLiteralName "HasSeenPlayer?") (Class|MyFPSCPPAICharacter|GetHasDetectedPlayer))
      (AI|Components|Blackboard|SetValueasObject _blackboard (Utilities|Name|MakeLiteralName "TargetPlayer") (Class|MyFPSCPPAICharacter|GetTargetActor)))))

(event Custom|ResetBlackboardKey
  (Class|MyFPSCPPAICharacter|SetHasDetectedPlayer false)
  (Class|MyFPSCPPAICharacter|SetTargetActor))

(event Custom|SetControllerAndBlackBoard
  (bind _asbp_aicontroller (Utilities|Casting|CastToBP_AIController (AI|GetAIController self)))
  (Variables|Default|SetAIController _asbp_aicontroller)
  (Variables|Default|SetBlackBoard (AI|GetBlackboard _asbp_aicontroller))
  (bind _asmy_fps_cppplayer_state (Utilities|Casting|CastToMyFPS_CPPPlayerState (Variables|Default|GetPlayerState)))
  (EventDispatchers|BindEventtoOnScoreChanged _asmy_fps_cppplayer_state (delegate Custom|ResetBlackboardKey)))

(event EventTick
  (params (DeltaSeconds :type Float%20%28single-precision%29))
  (bind _blackboard (Variables|Default|GetBlackBoard))
  (Utilities|IsValid (Class|MyFPSCPPAICharacter|GetTargetActor)
    (:Is%20Valid
      _)
    (:Is%20Not%20Valid
      (Class|MyFPSCPPAICharacter|SetHasDetectedPlayer false)
      (Class|MyFPSCPPAICharacter|StopFire)))
  (Utilities|IsValid _blackboard
    (:Is%20Valid
      (AI|Components|Blackboard|SetValueasBool _blackboard (Utilities|Name|MakeLiteralName "HasSeenPlayer?") (Class|MyFPSCPPAICharacter|GetHasDetectedPlayer))
      (AI|Components|Blackboard|SetValueasObject _blackboard (Utilities|Name|MakeLiteralName "TargetPlayer") (Class|MyFPSCPPAICharacter|GetTargetActor)))))

(fn ConstructionScript)